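; BP_Follow is a GOAP action that makes an NPC follow a target actor.
; Its procedural precondition takes the first entry of the pawn's target list as the target and always returns true, without checking for an empty list.
; Performing it writes the action name onto the GOAPNPC2 pawn and issues a MoveToActor through its AI controller.
; It returns false after issuing the move, so it never reports completion.
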(fn PerformAction
  (params (pawn :type Pawn%20Object%20Reference))
  (bind _asgoapnpc2 (Utilities|Casting|CastToGOAPNPC2 pawn))
  (Variables|/Game/NPC/Blueprints/GOAPNPC2.GOAPNPC2_C|SetActionName _asgoapnpc2 (Variables|Default|Getname))
  (bind _returnvalue (Class|GOAPAction|GetTarget))
  (bind _asaicontroller (Utilities|Casting|CastToAIController (Pawn|GetController pawn)))
  (AI|Navigation|MovetoActor _asaicontroller _returnvalue -1.0 true true true 0)
  (return false))

(fn CheckProceduralPrecondition
  (params (pawn :type Pawn%20Object%20Reference))
  (bind _returnvalue (Class|GOAPAction|GetTargetsList pawn))
  (Class|GOAPAction|SetTarget (Utilities|Array|Get(acopy) _returnvalue))
  (return true))