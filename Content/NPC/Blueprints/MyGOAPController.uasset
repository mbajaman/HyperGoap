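; GOAP AI controller for NPCs that runs goal-oriented action planning and shows the resulting plan on screen.
; Tick runs ExecuteGOAP behind a 0.3-second Delay, throttling how often planning happens.
; On success it fetches the plan, joins the action names in reverse order with arrows, and prints the string under a fixed key for debugging.
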(event EventTick
  (params (DeltaSeconds :type Float%20%28single-precision%29))
  (Utilities|FlowControl|Delay 0.3)
  (bind _returnvalue (Class|GOAPController|ExecuteGOAP))
  (if _returnvalue
    (bind _returnvalue_2 (Class|GOAPController|GetPlan))
    (Variables|Default|SetPlan "")
    (bind _arrayelement (Utilities|Array|ReverseforEachLoop _returnvalue_2)
      (:LoopBody
        (Variables|Default|SetPlan (Utilities|String|Append (Utilities|String|Append (Variables|Default|GetPlan) "->") (Variables|/Script/HyperGoap.GOAPAction|Getname _arrayelement))))
      (:Completed
        (Development|PrintString (Variables|Default|GetPlan) true true "(R=0.000000,G=0.660000,B=1.000000,A=1.000000)" 2.0 "1")))))

(fn ConstructionScript)