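; BP_Log is a collectible log prop that GOAP NPCs gather by bumping into it.
; On a Hit event from a GOAPNPC, a DoOnce gate lets it increment that NPC's CollectedLogs count a single time, then the log destroys itself.
; A disconnected branch that would credit BP_FirstPersonCharacter the same way remains in the graph but never runs.
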(event Collision|EventHit
  (params (MyComp :type Primitive%20Component%20Object%20Reference) (Other :type Actor%20Object%20Reference) (OtherComp :type Primitive%20Component%20Object%20Reference) (bSelfMoved :type Boolean) (HitLocation :type Vector :default "0, 0, 0") (HitNormal :type Vector :default "0, 0, 0") (NormalImpulse :type Vector :default "0, 0, 0") (Hit :type Hit%20Result%20Structure%20%28by%20ref%29))
  (bind _asgoapnpc (Utilities|Casting|CastToGOAPNPC Other))
  (Utilities|FlowControl|DoOnce false
    (:Completed
      (Variables|/Game/NPC/Blueprints/GOAPNPC.GOAPNPC_C|SetCollected%20Logs _asgoapnpc (+ (Variables|/Game/NPC/Blueprints/GOAPNPC.GOAPNPC_C|GetCollected%20Logs _asgoapnpc) 1))
      (Actor|DestroyActor self))))

(fn ConstructionScript)